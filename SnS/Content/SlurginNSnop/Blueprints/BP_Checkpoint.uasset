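; BP_Checkpoint is a checkpoint actor that records itself as the latest checkpoint when Snop or Slurgin enters its trigger.
; The Trigger overlap checks the other actor for an exact class match with BP_Snop or BP_Slurgin.
; Either match writes this actor to LastCheckpoint on the SnS game mode and plays a 2D sine-tone ping, with no guard against repeat activation.
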(event OnComponentBeginOverlap(Trigger)
  (params (OverlappedComponent :type Primitive%20Component%20Object%20Reference) (OtherActor :type Actor%20Object%20Reference) (OtherComp :type Primitive%20Component%20Object%20Reference) (OtherBodyIndex :type Integer) (bFromSweep :type Boolean) (SweepResult :type Hit%20Result%20Structure%20%28by%20ref%29))
  (if (== (Utilities|GetClass OtherActor) "/Game/SlurginNSnop/Blueprints/BP_Snop.BP_Snop_C")
    (Utilities|Casting|CastToBP_Snop OtherActor)
    (bind _assn_s (Utilities|Casting|CastToSnS (Game|GetGameMode) :!label _label))
    (Variables|/Game/Gamemodes/SnS.SnS_C|SetlastCheckpoint _assn_s self)
    (Audio|PlaySound2D "/Engine/EngineSounds/1kSineTonePing.1kSineTonePing" 1.0 1.0 0.0 0 0)
    (elif (== (Utilities|GetClass OtherActor) "/Game/ChaseAssets/SlimeShot/BP_Slurgin.BP_Slurgin_C")
      (Utilities|Casting|CastToBP_Slurgin OtherActor)
      (goto _label))))

(event EventBeginPlay)

(event Collision|EventActorBeginOverlap
  (params (OtherActor :type Actor%20Object%20Reference)))

(event EventTick
  (params (DeltaSeconds :type Float%20%28single-precision%29)))

(fn ConstructionScript)