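; Bug enemy that detects and harms the two player characters, Slurgin and Snop.
; PawnSensing sets the "hasSeenPlayer?" Blackboard flag on sighting either character, then clears it after a 15-second task delay.
; Sphere overlap kills the bug with an explosion effect when hit by a SlimeBall, a bashing Snop or a fast-rolling shelled Snop.
; Otherwise, touching either character records it in BP_Respawn and applies damage.
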(event OnSeePawn(PawnSensing)
  (params (Pawn :type Pawn%20Object%20Reference))
  (Utilities|Casting|CastToBP_Slurgin Pawn
    (:then
      (AI|Components|Blackboard|SetValueasBool (AI|GetBlackboard (AI|GetAIController self)) (Utilities|Name|MakeLiteralName "hasSeenPlayer?") true))
    (:CastFailed
      (Utilities|Casting|CastToBP_Snop Pawn)
      (AI|Components|Blackboard|SetValueasBool (AI|GetBlackboard (AI|GetAIController self)) (Utilities|Name|MakeLiteralName "hasSeenPlayer?") true)))
  (GameplayTasks|TaskWaitDelay (AI|GetAIController self) 15.0
    (:OnFinish
      (AI|Components|Blackboard|SetValueasBool (AI|GetBlackboard (AI|GetAIController self)) (Utilities|Name|MakeLiteralName "hasSeenPlayer?") false))))

(event OnComponentBeginOverlap(Sphere1)
  (params (OverlappedComponent :type Primitive%20Component%20Object%20Reference) (OtherActor :type Actor%20Object%20Reference) (OtherComp :type Primitive%20Component%20Object%20Reference) (OtherBodyIndex :type Integer) (bFromSweep :type Boolean) (SweepResult :type Hit%20Result%20Structure%20%28by%20ref%29))
  ;[1 1 1] BugCollision
  (if (== (Utilities|GetClass OtherActor) "/Game/ChaseAssets/SlimeShot/SlimeBall.SlimeBall_C")
    (Utilities|Casting|CastToSlimeBall OtherActor)
    (CallFunction|CustomHitEvent :!label _label)
    (elif (== (Utilities|GetClass OtherActor) "/Game/ChaseAssets/SlimeShot/BP_Slurgin.BP_Slurgin_C")
      (bind _asbp_slurgin (Utilities|Casting|CastToBP_Slurgin OtherActor))
      (bind _returnvalue (Actor|GetActorOfClass "/Game/SlurginNSnop/Blueprints/BP_Respawn.BP_Respawn_C"))
      (Variables|/Game/SlurginNSnop/Blueprints/BP_Respawn.BP_Respawn_C|SetkilledCharacter _returnvalue "/Game/ChaseAssets/SlimeShot/BP_Slurgin.BP_Slurgin_C")
      (Game|Damage|ApplyDamage _asbp_slurgin 1.0 0 0)
      (else
        (bind _asbp_snop (Utilities|Casting|CastToBP_Snop OtherActor))
        (if (or (Variables|/Game/SlurginNSnop/Blueprints/BP_Snop.BP_Snop_C|GetisBash _asbp_snop) (and (Variables|/Game/SlurginNSnop/Blueprints/BP_Snop.BP_Snop_C|GetisShell _asbp_snop) (>= (Variables|/Game/SlurginNSnop/Blueprints/BP_Snop.BP_Snop_C|GetRollingSpeed _asbp_snop) 1e+02)))
          (goto _label)
          (else
            (bind _returnvalue_2 (Actor|GetActorOfClass "/Game/SlurginNSnop/Blueprints/BP_Respawn.BP_Respawn_C"))
            (Variables|/Game/SlurginNSnop/Blueprints/BP_Respawn.BP_Respawn_C|SetkilledCharacter _returnvalue_2 "/Game/SlurginNSnop/Blueprints/BP_Snop.BP_Snop_C")
            (Game|Damage|ApplyDamage _asbp_snop 1.0 0 0)))))))

(event Custom|CustomHit_Event
  ;[1 1 1] DIE
  (Niagara|SpawnSystematLocation "/Game/ChaseAssets/Bug/BugExplosionSystem.BugExplosionSystem" (Transformation|GetActorLocation))
  (Actor|DestroyActor))

(fn ConstructionScript)