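; BP_WorldController removes tagged BP_SaltedCopper actors when the bug kill count reaches set thresholds.
; Its BugDestroyed event reads BugKillCount, destroying "Bug" tagged actors at the first threshold and "Bug2" tagged actors at the second.
; The "Bug2" check is nested inside the "Bug" loop, so it only runs while "Bug" tagged actors are still found.
; The event does not increment the count itself.
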(event Custom|BugDestroyed
  (bind _outactors (Actor|GetAllActorsOfClasswithTag "/Game/SlurginNSnop/Blueprints/BP_SaltedCopper.BP_SaltedCopper_C" "Bug"))
  (for _array_element _outactors
    (if (== (Variables|Default|GetBugKillCount) 2)
      (Actor|DestroyActor _array_element)
      (else
        (bind _outactors_2 (Actor|GetAllActorsOfClasswithTag "/Game/SlurginNSnop/Blueprints/BP_SaltedCopper.BP_SaltedCopper_C" "Bug2"))
        (for _array_element_2 _outactors_2
          (if (== (Variables|Default|GetBugKillCount) 4)
            (Actor|DestroyActor _array_element_2)))))))