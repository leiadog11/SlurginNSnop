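; BP_AI is a bug AI pawn that reacts to seeing player pawns and explodes when hit by slime.
; Pawn sensing of a BP_Slurgin or BP_Snop sets the blackboard's "hasSeenPlayer?" flag, then a timed wait task clears it.
; A SlimeBall overlapping its sphere calls a custom hit event, which spawns an explosion effect and destroys the bug.
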(event OnSeePawn(PawnSensing)
  (params (Pawn :type Pawn%20Object%20Reference))
  (Utilities|Casting|CastToBP_Slurgin Pawn
    (:then
      (AI|Components|Blackboard|SetValueasBool (AI|GetBlackboard (AI|GetAIController self)) (Utilities|Name|MakeLiteralName "hasSeenPlayer?") true))
    (:CastFailed
      (Utilities|Casting|CastToBP_Snop Pawn)
      (AI|Components|Blackboard|SetValueasBool (AI|GetBlackboard (AI|GetAIController self)) (Utilities|Name|MakeLiteralName "hasSeenPlayer?") true)))
  (GameplayTasks|TaskWaitDelay (AI|GetAIController self) 15.0
    (:OnFinish
      (AI|Components|Blackboard|SetValueasBool (AI|GetBlackboard (AI|GetAIController self)) (Utilities|Name|MakeLiteralName "hasSeenPlayer?") false))))

(event OnComponentBeginOverlap(Sphere1)
  (params (OverlappedComponent :type Primitive%20Component%20Object%20Reference) (OtherActor :type Actor%20Object%20Reference) (OtherComp :type Primitive%20Component%20Object%20Reference) (OtherBodyIndex :type Integer) (bFromSweep :type Boolean) (SweepResult :type Hit%20Result%20Structure%20%28by%20ref%29))
  (Utilities|Casting|CastToSlimeBall OtherActor)
  (CallFunction|CustomHitEvent))

(event Custom|CustomHit_Event
  (Niagara|SpawnSystematLocation "/Game/ChaseAssets/Bug/BugExplosionSystem.BugExplosionSystem" (Transformation|GetActorLocation))
  (Actor|DestroyActor))

(fn ConstructionScript)