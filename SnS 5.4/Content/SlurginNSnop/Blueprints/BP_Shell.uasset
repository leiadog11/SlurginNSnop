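; BP_Shell is a player-controlled shell form that turns back into BP_Snop when E is pressed.
; On E, it spawns a Snop at the Shell component's location with the actor's rotation and scale, hands possession to it, then destroys itself.
; Only mouse yaw drives the camera input; gamepad look and mouse pitch events are empty, with their input nodes left disconnected.
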(event Input|AxisEvents|InputAxisTurnRight/LeftGamepad
  (params (AxisValue :type Float%20%28single-precision%29))
  ;[0.05098 0.05098 0.05098] Camera Input - Gamepad
)

(event Input|AxisEvents|InputAxisTurnRight/LeftMouse
  (params (AxisValue :type Float%20%28single-precision%29))
  ;[0.05098 0.05098 0.05098] Camera Input - Mouse
  (Pawn|Input|AddControllerYawInput AxisValue))

(event Input|AxisEvents|InputAxisLookUp/DownMouse
  (params (AxisValue :type Float%20%28single-precision%29))
  ;[0.05098 0.05098 0.05098] Camera Input - Mouse
)

(event Input|AxisEvents|InputAxisLookUp/DownGamepad
  (params (AxisValue :type Float%20%28single-precision%29))
  ;[0.05098 0.05098 0.05098] Camera Input - Gamepad
)

(event Input|KeyboardEvents|E
  (params (Key :type Key%20Structure :default "None"))
  ;[1 1 1] Change to Snop
  (:Pressed
    (bind _returnvalue (Game|SpawnActorfromClass "/Game/SlurginNSnop/Blueprints/BP_Snop.BP_Snop_C" (Math|Transform|MakeTransform (Transformation|GetWorldLocation (Variables|Default|GetShell)) (Transformation|GetActorRotation) (Transformation|GetActorScale3D)) "AlwaysSpawn" "MultiplyWithRoot" 0 0))
    (Pawn|Possess (Game|GetPlayerController (Variables|GetPlayerState)) _returnvalue)
    (Actor|DestroyActor)))

(fn ConstructionScript)