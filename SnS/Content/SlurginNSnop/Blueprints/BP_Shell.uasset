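; BP_Shell is a player-controlled shell form that swaps to BP_Snop on E by spawning it, possessing it and destroying itself.
; Tick measures rolling speed from the sphere's physics velocity, and Z allows a bash only at zero speed.
; The bash briefly lunges and tilts the shell with delays while enabling HITBOX collision, whose hit event is empty.
; Only mouse yaw drives the camera; pitch and gamepad look are unconnected.
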(event OnComponentHit(HITBOX)
  (params (HitComponent :type Primitive%20Component%20Object%20Reference) (OtherActor :type Actor%20Object%20Reference) (OtherComp :type Primitive%20Component%20Object%20Reference) (NormalImpulse :type Vector :default "0, 0, 0") (Hit :type Hit%20Result%20Structure%20%28by%20ref%29)))

(event EventTick
  (params (DeltaSeconds :type Float%20%28single-precision%29))
  ;[1 1 1] Rolling Speed
  (bind _returnvalue (Physics|GetPhysicsLinearVelocity (Variables|Default|GetSphere) "None"))
  (Variables|Default|SetRollingSpeed (Math|Vector|VectorLength _returnvalue)))

(event Input|AxisEvents|InputAxisTurnRight/LeftGamepad
  (params (AxisValue :type Float%20%28single-precision%29))
  ;[0.05098 0.05098 0.05098] Camera Input - Gamepad
)

(event Input|AxisEvents|InputAxisTurnRight/LeftMouse
  (params (AxisValue :type Float%20%28single-precision%29))
  ;[0.05098 0.05098 0.05098] Camera Input - Mouse
  (Pawn|Input|AddControllerYawInput AxisValue))

(event Input|AxisEvents|InputAxisLookUp/DownMouse
  (params (AxisValue :type Float%20%28single-precision%29))
  ;[0.05098 0.05098 0.05098] Camera Input - Mouse
)

(event Input|AxisEvents|InputAxisLookUp/DownGamepad
  (params (AxisValue :type Float%20%28single-precision%29))
  ;[0.05098 0.05098 0.05098] Camera Input - Gamepad
)

(event Input|KeyboardEvents|E
  (params (Key :type Key%20Structure :default "None"))
  ;[1 1 1] Change to Snop
  (:Pressed
    (bind _returnvalue (Game|SpawnActorfromClass "/Game/SlurginNSnop/Blueprints/BP_Snop.BP_Snop_C" (Math|Transform|MakeTransform (Transformation|GetWorldLocation (Variables|Default|GetShell)) (Transformation|GetActorRotation) (Transformation|GetActorScale3D)) "AlwaysSpawn" "MultiplyWithRoot" 0 0))
    (Pawn|Possess (Game|GetPlayerController (Variables|GetPlayerState)) _returnvalue)
    (Actor|DestroyActor)))

(event Input|KeyboardEvents|Z
  (params (Key :type Key%20Structure :default "None"))
  (bind _shell (Variables|Default|GetShell))
  (bind _shell_2 (Variables|Default|GetShell))
  (:Pressed
    (if (and (Variables|Default|GetCanBash) (== (Variables|Default|GetRollingSpeed) 0.0))
      (Variables|Default|SetCanBash false)
      (Transformation|AddRelativeLocation _shell (Math|Vector|MakeVector 2e+01 0.0 0.0) false false)
      (Transformation|AddRelativeRotation _shell "0.000000,0.000000,30.000000" false false)
      (Collision|SetCollisionEnabled (Variables|Default|GetHITBOX) "QueryAndPhysics")
      (Utilities|FlowControl|Delay 0.2)
      (Transformation|AddRelativeLocation _shell_2 (Math|Vector|MakeVector -2e+01 0.0 0.0) false false)
      (Transformation|AddRelativeRotation _shell_2 "0.000000,0.000000,-30.000000" false false)
      (Utilities|FlowControl|Delay 0.2)
      (Collision|SetCollisionEnabled (Variables|Default|GetHITBOX) "NoCollision")
      (Variables|Default|SetCanBash true))))

(fn ConstructionScript)