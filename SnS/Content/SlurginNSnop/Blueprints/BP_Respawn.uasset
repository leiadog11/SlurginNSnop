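; BP_Respawn handles respawning of the two player characters, Snop and Slurgin, at the saved checkpoint.
; RespawnPlayer destroys the first actor found of the KilledCharacter class, then spawns a fresh copy at the checkpoint's RespawnPos, ignoring collisions.
; The new pawn is possessed by a fixed local controller: player 0 for Snop, player 1 for Slurgin.
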(event Custom|RespawnPlayer
  (bind _killedcharacter (Variables|Default|GetkilledCharacter))
  (bind _savedcheckpoint (Variables|Default|GetsavedCheckpoint))
  (bind _respawnpos (Variables|/Game/SlurginNSnop/Blueprints/BP_Checkpoint.BP_Checkpoint_C|GetRespawnPos _savedcheckpoint))
  (bind _returnvalue (Transformation|GetWorldTransform _respawnpos))
  (bind _returnvalue_2 (Actor|GetActorOfClass _killedcharacter))
  (Actor|DestroyActor _returnvalue_2)
  (if (== _killedcharacter "/Game/SlurginNSnop/Blueprints/BP_Snop.BP_Snop_C")
    (bind _returnvalue_3 (Game|SpawnActorfromClass "/Game/SlurginNSnop/Blueprints/BP_Snop.BP_Snop_C" (Math|Transform|MakeTransform (.location _returnvalue) (.rotation _returnvalue) "1.000000,1.000000,1.000000") "AlwaysSpawn" "MultiplyWithRoot" 0 0))
    (Pawn|Possess (Game|GetPlayerController 0) _returnvalue_3)
    (elif (== _killedcharacter "/Game/ChaseAssets/SlimeShot/BP_Slurgin.BP_Slurgin_C")
      (bind _returnvalue_4 (Game|SpawnActorfromClass "/Game/ChaseAssets/SlimeShot/BP_Slurgin.BP_Slurgin_C" (Math|Transform|MakeTransform (.location _returnvalue) (.rotation _returnvalue) "1.000000,1.000000,1.000000") "AlwaysSpawn" "MultiplyWithRoot" 0 0))
      (Pawn|Possess (Game|GetPlayerController 1) _returnvalue_4))))

(fn ConstructionScript)