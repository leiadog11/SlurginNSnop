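; Breakable wall covered in plants that takes two stages to destroy.
; A SlimeBall hitting the Box component destroys the five plant components and flags the plants as destroyed.
; Once they are gone, a BP_Snop that begins overlapping the wall at a high enough RollingSpeed destroys the whole actor.
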(event OnComponentHit(Box)
  (params (HitComponent :type Primitive%20Component%20Object%20Reference) (OtherActor :type Actor%20Object%20Reference) (OtherComp :type Primitive%20Component%20Object%20Reference) (NormalImpulse :type Vector :default "0, 0, 0") (Hit :type Hit%20Result%20Structure%20%28by%20ref%29))
  (if (== (Utilities|GetClass OtherActor) "/Game/ChaseAssets/SlimeShot/SlimeBall.SlimeBall_C")
    (Components|DestroyComponent (Variables|Default|GetPlants))
    (Components|DestroyComponent (Variables|Default|GetPlants1))
    (Components|DestroyComponent (Variables|Default|GetPlants2))
    (Components|DestroyComponent (Variables|Default|GetPlants3))
    (Components|DestroyComponent (Variables|Default|GetPlants4))
    (Variables|Default|SetarePlansDestroyed true)))

(event Collision|EventActorBeginOverlap
  (params (OtherActor :type Actor%20Object%20Reference))
  ;[1 1 1] Break Wall
  (if (Variables|Default|GetarePlansDestroyed)
    (bind _asbp_snop (Utilities|Casting|CastToBP_Snop OtherActor)
      (:then
        (if (>= (Variables|/Game/SlurginNSnop/Blueprints/BP_Snop.BP_Snop_C|GetRollingSpeed _asbp_snop) 2e+02)
          (Actor|DestroyActor)))
      (:CastFailed
        (Development|PrintText "CAST FAILED")))))

(fn ConstructionScript)